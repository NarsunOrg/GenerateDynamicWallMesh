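; BP_DoorFrame is a door frame actor from the house generation drop-to-world set, with mouse-drag yaw rotation logic.
; MouseMove yaws the DoorFrame component by the negated horizontal mouse delta while CanRotate is true, then stores the new mouse location.
; EndRotate clears CanRotate, but StartRotate is empty and the nodes that would set it and seed the start location are disconnected.
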(event Custom|Mouse%20Move
  (params (MouseLocation :type Vector%202D%20Structure))
  (if (Variables|Default|GetCanRotate)
    (Transformation|AddWorldRotation (Variables|Default|GetDoorFrame) (Math|Rotator|MakeRotator 0.0 0.0 (* (.X (Math|Vector2D|BreakVector2D (- MouseLocation (Variables|Default|GetStartRotateLocation)))) -1.0)) false false)
    (Variables|Default|SetStartRotateLocation MouseLocation)))

(event Custom|Start%20Rotate
  (params (MouseLocation :type Vector%202D%20Structure)))

(event Custom|End%20Rotate
  (Variables|Default|SetCanRotate false))

(event EventBeginPlay)

(event Collision|EventActorBeginOverlap
  (params (OtherActor :type Actor%20Object%20Reference)))

(event EventTick
  (params (DeltaSeconds :type Float%20%28single-precision%29)))

(fn ConstructionScript)