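; Transform gizmo actor for moving scene components with the mouse along colored X, Y and Z arrows, which highlight yellow on hover.
; Right-click alternately attaches the traced component to the gizmo root or detaches it, toggling gizmo visibility.
; M toggles move mode, where left-click traces record grab distance and axis.
; Tick projects the cursor offset onto that axis to move the root, or yaws the Rotation handle from mouse delta.
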(event OnBeginCursorOver(X)
  (params (TouchedComponent :type Primitive%20Component%20Object%20Reference))
  ;[1 1 1] Hightlighting Arrow By Yellow Material
  (Rendering|Material|SetMaterial (Variables|Default|GetX) 0 "/Game/My_Working/HouseGeneration/Mat/YellowMaterial.YellowMaterial")
  (Utilities|FlowControl|Gate true) ; enters at Open
)

(event OnBeginCursorOver(Y)
  (params (TouchedComponent :type Primitive%20Component%20Object%20Reference))
  ;[1 1 1] Hightlighting Arrow By Yellow Material
  (Rendering|Material|SetMaterial (Variables|Default|GetY) 0 "/Game/My_Working/HouseGeneration/Mat/YellowMaterial.YellowMaterial")
  (Utilities|FlowControl|Gate true) ; enters at Open
)

(event OnBeginCursorOver(Z)
  (params (TouchedComponent :type Primitive%20Component%20Object%20Reference))
  ;[1 1 1] Hightlighting Arrow By Yellow Material
  (Rendering|Material|SetMaterial (Variables|Default|GetZ) 0 "/Game/My_Working/HouseGeneration/Mat/YellowMaterial.YellowMaterial")
  (Utilities|FlowControl|Gate true) ; enters at Open
)

(event OnEndCursorOver(X)
  (params (TouchedComponent :type Primitive%20Component%20Object%20Reference))
  ;[1 1 1] Hightlighting Arrow By Yellow Material
  (Rendering|Material|SetMaterial (Variables|Default|GetX) 0 "/Game/My_Working/HouseGeneration/Mat/RedColor.RedColor")
  (Utilities|FlowControl|Gate true) ; enters at Close
)

(event OnEndCursorOver(Y)
  (params (TouchedComponent :type Primitive%20Component%20Object%20Reference))
  ;[1 1 1] Hightlighting Arrow By Yellow Material
  (Rendering|Material|SetMaterial (Variables|Default|GetY) 0 "/Game/My_Working/HouseGeneration/Mat/GreenColor.GreenColor")
  (Utilities|FlowControl|Gate true) ; enters at Close
)

(event OnEndCursorOver(Z)
  (params (TouchedComponent :type Primitive%20Component%20Object%20Reference))
  ;[1 1 1] Hightlighting Arrow By Yellow Material
  (Rendering|Material|SetMaterial (Variables|Default|GetZ) 0 "/Game/My_Working/HouseGeneration/Mat/BlueColor.BlueColor")
  (Utilities|FlowControl|Gate true) ; enters at Close
)

(event EventBeginPlay
  ;[1 1 1] Enable Input For Gizmo
  (Input|EnableInput (Game|GetPlayerController 0)))

(event EventTick
  (params (DeltaSeconds :type Float%20%28single-precision%29))
  ;[1 1 1] Moving Gizmo
  (switch Utilities|FlowControl|Switch|SwitchonEnum_AxisVariable (.xyz (Utilities|Struct|MakeS_DraggedAxis 0 (CallFunction|GrabbedAxisComponentCheck (Variables|Default|GetAxisDragged))))
    (:NewEnumerator0
      (Utilities|IsValid (Variables|Default|GetAxisDragged) :!label _label
        (:Is%20Valid
          (CallFunction|Movement))))
    (:NewEnumerator1
      (goto _label))
    (:NewEnumerator2
      (goto _label))
    (:NewEnumerator3
      (Transformation|AddLocalRotation (Variables|Default|GetRotation) (Math|Rotator|MakeRotator 0.0 0.0 (* (.DeltaX (Class|PlayerController|GetInputMouseDelta (Game|GetPlayerController 0))) -1e+01)) false false))))

(event Input|MouseEvents|LeftMouseButton
  (params (Key :type Key%20Structure))
  (bind _returnvalue (Game|GetPlayerController 0))
  (bind (_worldlocation _worlddirection) (Game|Player|ConvertMouseLocationToWorldSpace _returnvalue))
  ;[1 1 1] Moving Attached Item
  (:Pressed
    (if (Variables|Default|GetEnableToMove)
      (bind _outhit (Collision|LineTraceByChannel _worldlocation (+ _worldlocation (* _worlddirection (Math|Vector|MakeVector 1e+04 1e+04 1e+04))) "TraceTypeQuery1" true 0 "Persistent"))
      (Variables|Default|SetDistanceToGrab (.Distance (Collision|BreakHitResult _outhit)))
      (switch Utilities|FlowControl|Switch|SwitchonEnum_AxisVariable (.xyz (Utilities|Struct|MakeS_DraggedAxis 0 (CallFunction|GrabbedAxisComponentCheck (.HitComponent (Collision|BreakHitResult _outhit)))))
        (:NewEnumerator0
          (Development|PrintString "X"))
        (:NewEnumerator1
          (Development|PrintString "Y"))
        (:NewEnumerator2
          (Development|PrintString "Z")))
      (Variables|Default|SetDrag%20Location (Math|Transform|InverseTransformLocation (Math|Conversions|ToTransform(Vector) (Math|Conversions|ToVector(Float) (Class|GameplayStatics|GetWorldOriginLocation))) (.Location (Collision|BreakHitResult _outhit))))))
  (:Released
    (if (Variables|Default|GetEnableToMove)
      (Variables|Default|SetAxisDragged 0))))

(event Input|KeyboardEvents|M
  (params (Key :type Key%20Structure))
  (bind _returnvalue (Game|GetPlayerController 0))
  ;[1 1 1] Enable Gizmo Axis
  (:Pressed
    (Variables|Default|SetEnableToMove (not (Variables|Default|GetEnableToMove)))
    (Variables|/Script/Engine.PlayerController|SetbShowMouseCursor _returnvalue (Variables|/Script/Engine.PlayerController|GetbShowMouseCursor _returnvalue))))

(event Input|MouseEvents|RightMouseButton
  (params (Key :type Key%20Structure))
  (bind _returnvalue (Game|GetPlayerController 0))
  (bind (_worldlocation _worlddirection) (Game|Player|ConvertMouseLocationToWorldSpace _returnvalue))
  ;[1 1 1] Attach & Deattach gizmo on the object you want to move by right click on the object
  (:Pressed
    (bind _outhit (Collision|LineTraceByChannel _worldlocation (+ _worldlocation (* _worlddirection "10000.000000,10000.000000,10000.000000")) "TraceTypeQuery1" false 0 "None"))
    (Utilities|FlowControl|FlipFlop
      (:A
        (Rendering|SetVisibility (Variables|Default|GetGizmoRoot) true true)
        (Transformation|SetWorldLocation (Variables|Default|GetGizmoRoot) (Math|Vector|MakeVector (.x (Transformation|GetWorldLocation (.HitComponent (Collision|BreakHitResult _outhit)))) (.y (Transformation|GetWorldLocation (.HitComponent (Collision|BreakHitResult _outhit)))) (Variables|Default|GetGizmoHeight)) false false)
        (Transformation|AttachComponentToComponent (.HitComponent (Collision|BreakHitResult _outhit)) (Variables|Default|GetGizmoRoot) "None" "KeepWorld" "KeepWorld" "KeepWorld" true))
      (:B
        (Transformation|DetachFromComponent (.HitComponent (Collision|BreakHitResult _outhit)) "KeepWorld" "KeepRelative" "KeepWorld" true)
        (Rendering|SetVisibility (Variables|Default|GetGizmoRoot) false true)))))

(fn ConstructionScript)

(fn GrabbedAxisComponentCheck
  (params (AxisComponent :type Primitive%20Component%20Object%20Reference))
  (Variables|Default|SetAxisDragged AxisComponent)
  (if (== (Variables|Default|GetAxisDragged) (Variables|Default|GetX))
    (return "NewEnumerator0")
    (elif (== (Variables|Default|GetAxisDragged) (Variables|Default|GetY))
      (return "NewEnumerator1")
      (elif (== (Variables|Default|GetAxisDragged) (Variables|Default|GetZ))
        (return "NewEnumerator2")
        (elif (== (Variables|Default|GetAxisDragged) (Variables|Default|GetRotation))
          (return "NewEnumerator3"))))))

(fn Movement
  (bind _returnvalue (Game|GetPlayerController 0))
  (bind _distancetograb (Variables|Default|GetDistanceToGrab))
  (bind (_worldlocation _worlddirection) (Game|Player|ConvertMouseLocationToWorldSpace _returnvalue))
  (Transformation|AddRelativeLocation (Variables|Default|GetGizmoRoot) (/ (Math|Vector|ProjectVectorontoVector (Math|Transform|InverseTransformLocation (Math|Conversions|ToTransform(Vector) (Variables|Default|GetDrag%20Location)) (+ _worldlocation (* _worlddirection (Math|Vector|MakeVector _distancetograb _distancetograb _distancetograb)))) (Math|Vector|GetForwardVector (Variables|Default|GetAxisDragged))) "50.000000,50.000000,50.000000") false false))