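; BP_WallInstance generates a row of instanced wall meshes from the initial and release locations stored on the character.
; WallGeneration adds an instanced static mesh component with query and physics collision, then loops up to the rounded release Y coordinate, placing world-space instances.
; Each step offsets along Y, but adds the whole new position to the running location, so spacing compounds.
; The construction script is empty.
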(fn ConstructionScript)

(fn WallGeneration
  (bind _mycharacter (Variables|WallGeneration|GetMyCharacter))
  (LocalVariables|SetInitiatialLocation (Variables|/Game/My_Working/HouseGeneration/MyArcVizCharacter.MyArcVizCharacter_C|GetInitialLocation _mycharacter))
  (LocalVariables|SetReleaseLocation (Variables|/Game/My_Working/HouseGeneration/MyArcVizCharacter.MyArcVizCharacter_C|GetReleaseLocation _mycharacter))
  (bind _returnvalue (AddComponent|AddInstancedStaticMeshComponent false))
  (bind _output_get (Variables|WallGeneration|SetInstanceStaticMesh _returnvalue))
  (Components|StaticMesh|SetStaticMesh _output_get (Variables|WallGeneration|GetWallMesh))
  (Collision|SetCollisionEnabled _output_get "QueryAndPhysics")
  (for _index (range 0 (Math|Float|Round (.y (LocalVariables|GetReleaseLocation))))
    (bind _output_get_2 (LocalVariables|SetCurrentLocation (+ (LocalVariables|GetInitiatialLocation) "0,10.000000,0")))
    (Components|InstancedStaticMesh|AddInstance (Variables|WallGeneration|GetInstanceStaticMesh) (Math|Transform|MakeTransform _output_get_2 "0, 0, 0" "1.000000,1.000000,1.000000") true)
    (LocalVariables|SetInitiatialLocation (+ (LocalVariables|GetInitiatialLocation) (LocalVariables|GetCurrentLocation)))))