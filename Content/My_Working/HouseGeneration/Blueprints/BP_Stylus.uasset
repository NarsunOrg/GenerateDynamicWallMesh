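; BP_Stylus is a house-generation tool that turns the player character's initial and release points into a wall.
; It caches MyArcVizCharacter on BeginPlay and copies that character's current location each Tick.
; FindingLengthAndGenerating draws a debug trace between both points, converts their distance into a mesh-relative scale and passes it to BP_WallGeneration's GenerateMesh.
; WallGeneration and InstanceMeshesSpawn are empty, with older spawning and instanced-mesh attempts left disconnected.
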(event EventBeginPlay
  (bind _asmy_arc_viz_character (Utilities|Casting|CastToMyArcVizCharacter (Game|GetPlayerCharacter 0)))
  (Variables|Default|SetMyCharacterRef _asmy_arc_viz_character))

(event EventTick
  (params (DeltaSeconds :type Float%20%28single-precision%29))
  (Variables|Default|SetActorPlaceLocation (Variables|/Game/My_Working/HouseGeneration/MyArcVizCharacter.MyArcVizCharacter_C|GetActorCurrentLocation (Variables|Default|GetMyCharacterRef))))

(fn ConstructionScript)

(fn WallGeneration)

(fn InstanceMeshesSpawn)

(fn FindingLengthandGenerating
  (bind _mycharacterref (Variables|Default|GetMyCharacterRef))
  (bind _output_get (LocalVariables|SetInitiatialLocation (Variables|/Game/My_Working/HouseGeneration/MyArcVizCharacter.MyArcVizCharacter_C|GetInitialLocation _mycharacterref)))
  (LocalVariables|SetCurrentLocation _output_get)
  (LocalVariables|SetReleaseLocation (Variables|/Game/My_Working/HouseGeneration/MyArcVizCharacter.MyArcVizCharacter_C|GetReleaseLocation _mycharacterref))
  (Collision|LineTraceByChannel (Math|Vector|MakeVector (.x (LocalVariables|GetInitiatialLocation)) (.y (LocalVariables|GetInitiatialLocation)) 1.5e+02) (Math|Vector|MakeVector (.x (LocalVariables|GetReleaseLocation)) (.y (LocalVariables|GetReleaseLocation)) 1.5e+02) "TraceTypeQuery1" true 0 "Persistent" true "(R=1.000000,G=0.000000,B=0.098436,A=1.000000)" "(R=1.000000,G=0.789766,B=0.000000,A=1.000000)" 1e+01)
  (bind _output_get_2 (Variables|Default|SetDistance (Math|Float|Round (Math|Vector|Distance(Vector) (LocalVariables|GetInitiatialLocation) (LocalVariables|GetReleaseLocation)))))
  (Development|PrintString (Utilities|String|ToString(Integer) _output_get_2) true true "(R=0.000000,G=0.660000,B=1.000000,A=1.000000)" 1.0)
  (bind _output_get_3 (LocalVariables|SetScale (/ (Variables|Default|GetDistance) (* (.y (.BoxExtent (Math|BoxSphereBounds|BreakBoxSphereBounds (StaticMesh|GetBounds (Variables|Default|GetWallMesh))))) 2.0))))
  (Development|PrintString (Utilities|String|ToString(Float) _output_get_3) true true "(R=1.000000,G=0.922361,B=0.000000,A=1.000000)" 1.0)
  (bind _returnvalue (Actor|GetActorOfClass "/Game/My_Working/HouseGeneration/Blueprints/BP_WallGeneration.BP_WallGeneration_C"))
  (Default|GenerateMesh _returnvalue (LocalVariables|GetScale) (LocalVariables|GetInitiatialLocation)))