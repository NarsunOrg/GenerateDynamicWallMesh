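; Spline-driven construction-script Blueprint for house generation that repeats a set of meshes at a fixed spacing along a spline.
; Each ItemStructure entry gets its own instanced static mesh component with a dynamic material instance.
; Straight-line distances between spline points, divided by RepeatWidth, set the instance count.
; A running counter places instances by distance along the spline, adding each entry's offset and rotation to the spline's.
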(fn ConstructionScript
  (CallFunction|FSplineGeneration))

(fn FSplineGeneration
  (bind _spline (Variables|Default|GetSpline))
  (bind _spline_2 (Variables|Default|GetSpline))
  (for _array_element (Variables|Default|GetItemStructure)
    (Variables|Default|SetLoopCount 0)
    (bind _returnvalue (AddComponent|AddInstancedStaticMeshComponent false))
    (Components|StaticMesh|SetStaticMesh _returnvalue (.StaticMesh (Utilities|Struct|BreakS_RepeatingItems _array_element)))
    (bind _returnvalue_2 (Rendering|Material|CreateDynamicMaterialInstance _returnvalue 0 (.Material (Utilities|Struct|BreakS_RepeatingItems _array_element)) "None" :!class /Script/Engine.PrimitiveComponent))
    (Rendering|Material|SetMaterial _returnvalue 0 _returnvalue_2)
    (for _index (range 0 (- (Spline|GetNumberOfSplinePoints _spline) 1))
      (for _index_2 (range 0 (- (.ReturnValue (Math|Float|Division(WholeandRemainder) (Math|Vector|Distance(Vector) (Spline|GetLocationatSplinePoint _spline _index "Local") (Spline|GetLocationatSplinePoint _spline (+ _index 1) "Local")) (Variables|Default|GetRepeatWidth))) 1))
        (Components|InstancedStaticMesh|AddInstance _returnvalue (Math|Transform|MakeTransform (Math|Vector|MakeVector (+ (.x (.Location (Math|Transform|BreakTransform (.Transform (Utilities|Struct|BreakS_RepeatingItems _array_element))))) (.x (Spline|GetLocationatDistanceAlongSpline _spline_2 (* (Variables|Default|GetLoopCount) (Variables|Default|GetRepeatWidth)) "Local"))) (+ (.y (.Location (Math|Transform|BreakTransform (.Transform (Utilities|Struct|BreakS_RepeatingItems _array_element))))) (.y (Spline|GetLocationatDistanceAlongSpline _spline_2 (* (Variables|Default|GetLoopCount) (Variables|Default|GetRepeatWidth)) "Local"))) (+ (.z (.Location (Math|Transform|BreakTransform (.Transform (Utilities|Struct|BreakS_RepeatingItems _array_element))))) (.z (Spline|GetLocationatDistanceAlongSpline _spline_2 (* (Variables|Default|GetLoopCount) (Variables|Default|GetRepeatWidth)) "Local")))) (Math|Rotator|MakeRotator (+ (.roll (.Rotation (Math|Transform|BreakTransform (.Transform (Utilities|Struct|BreakS_RepeatingItems _array_element))))) (.roll (Spline|GetRotationatDistanceAlongSpline _spline_2 (* (Variables|Default|GetLoopCount) (Variables|Default|GetRepeatWidth)) "Local"))) (+ (.pitch (.Rotation (Math|Transform|BreakTransform (.Transform (Utilities|Struct|BreakS_RepeatingItems _array_element))))) (.pitch (Spline|GetRotationatDistanceAlongSpline _spline_2 (* (Variables|Default|GetLoopCount) (Variables|Default|GetRepeatWidth)) "Local"))) (+ (.yaw (.Rotation (Math|Transform|BreakTransform (.Transform (Utilities|Struct|BreakS_RepeatingItems _array_element))))) (.yaw (Spline|GetRotationatDistanceAlongSpline _spline_2 (* (Variables|Default|GetLoopCount) (Variables|Default|GetRepeatWidth)) "Local")))) (.Scale (Math|Transform|BreakTransform (.Transform (Utilities|Struct|BreakS_RepeatingItems _array_element))))) false)
        (Math|Integer|IncrementInt (Variables|Default|GetLoopCount))))))