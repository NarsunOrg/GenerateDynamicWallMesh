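; Wall generator Blueprint for house generation that builds a box wall mesh and saves it into a static mesh asset.
; GenerateMesh appends a rotated Geometry Script box to its dynamic mesh, taking width and location as inputs and depth and height from variables.
; ConvertToStaicMesh copies the result into TargetMesh if valid, then GenerateMesh clears that reference and resets the dynamic mesh.
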(event Custom|GenerateMesh
  (params (Width :type Float%20%28single-precision%29) (Transform%20Location :type Vector))
  (bind _returnvalue (DynamicMeshComponent|GetDynamicMesh (Variables|DynamicMeshActor|GetDynamicMeshComponent)))
  (bind _output_get (Variables|Default|SetDynamicMesh _returnvalue))
  (Class|GeometryScriptLibraryMeshPrimitiveFunctions|AppendBox :TargetMesh _output_get :Transform (Math|Transform|MakeTransform Transform%20Location "0.000000,90.000000,0.000000" "1.000000,1.000000,1.000000") :DimensionX Width :DimensionY (Variables|Default|GetDepth) :DimensionZ (Variables|Default|GetHeight) :Debug 0)
  (CallFunction|ConverttoStaicMesh)
  (Variables|Default|SetTargetMesh 0)
  (DynamicMesh|Reset (Variables|Default|GetDynamicMesh)))

(fn ConstructionScript)

(fn ConverttoStaicMesh
  (bind _targetmesh (Variables|Default|GetTargetMesh)
    (:then
      (GeometryScript|StaticMesh|CopyMeshtoStaticMesh :FromDynamicMesh (Variables|Default|GetDynamicMesh) :ToStaticMeshAsset _targetmesh :Debug 0))
    (:else)))